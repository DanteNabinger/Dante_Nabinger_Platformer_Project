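; BP_Door is an interactable hinged door that alternately opens and closes each time INTInteract fires.
; On opening, UpdatedoorAngle uses a dot product of the door's forward vector and the direction to the player to choose a positive or negative 90-degree swing.
; A timeline lerps the Arrow component's relative yaw to that angle, and a FlipFlop reverses the timeline on the next interaction.
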(event `/Game/Interfaces/Interface_Interact.INT_Interact`
  (params (PlayerRef :type "/Game/Player/BP_PlayerChar Object Reference"))
  (`/Engine/EditorBlueprintResources/StandardMacros.FlipFlop`
    (:`A`
      (bind _returnvalue (`self.UpdatedoorAngle` PlayerRef))
      (bind (_direction _alpha) (`Timeline|Timeline` :!label _label)
        (:`Update`
          (`SceneComponent.K2_SetRelativeRotation` (`self.Arrow`) (`KismetMathLibrary.MakeRotator` 0.0 0.0 (`KismetMathLibrary.Lerp` 0.0 _returnvalue _alpha)) false false))))
    (:`B`
      (goto _label :!via `Reverse`))))

(fn `UpdatedoorAngle`
  (params (self2 :type "Actor Object Reference"))
  (returns (ReturnValue :type "Float (double-precision)"))
  (return (select `bool` (> (`KismetMathLibrary.Dot_VectorVector` (`KismetMathLibrary.GetDirectionUnitVector` (`self.K2_GetActorLocation`) (`self.K2_GetActorLocation` self2)) (`self.GetActorForwardVector`)) 0.0) :`false` -90.0 :`true` 90.0)))

(fn `UserConstructionScript`)